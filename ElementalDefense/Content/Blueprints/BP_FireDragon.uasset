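; Fire dragon wave enemy that follows a random left or right TargetPoint route to damage the base, fighting the player en route.
; Tick selects Patrol, Suspicious, Chase or Attack from the detection box, eye line trace, memory countdown and player distance.
; Attack fires projectiles at the player, while only non-fire player projectiles damage the dragon.
; Death awards the player a material; death or reaching the base updates the game mode's enemy count.
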(event OnComponentBeginOverlap(DetectionArea)
  (params (OverlappedComponent :type Primitive%20Component%20Object%20Reference) (OtherActor :type Actor%20Object%20Reference) (OtherComp :type Primitive%20Component%20Object%20Reference) (OtherBodyIndex :type Integer) (bFromSweep :type Boolean) (SweepResult :type Hit%20Result%20Structure%20%28by%20ref%29))
  ;[1 0.03917 0.07738] Detection Precess
  ;;[1 1 1] Detection Area Enter/Exit
  (bind _asfirst_person_character (Utilities|Casting|CastToFirstPersonCharacter OtherActor))
  (if (Variables|/Game/Blueprints/FirstPersonCharacter.FirstPersonCharacter_C|GetisDead _asfirst_person_character)
    (Variables|Default|SetIsSupecious false)
    (else
      (Variables|Default|SetIsSupecious true))))

(event OnComponentEndOverlap(DetectionArea)
  (params (OverlappedComponent :type Primitive%20Component%20Object%20Reference) (OtherActor :type Actor%20Object%20Reference) (OtherComp :type Primitive%20Component%20Object%20Reference) (OtherBodyIndex :type Integer))
  ;[1 0.03917 0.07738] Detection Precess
  ;;[1 1 1] Detection Area Enter/Exit
  (Utilities|Casting|CastToFirstPersonCharacter OtherActor)
  (Variables|Default|SetIsSupecious false)
  (Variables|Default|SetDetectionDelayTemp 0.1))

(event Custom|PlayerDetectedEvent
  (Variables|Default|SetIsInView true)
  (Variables|Default|SetDetectionDelayTemp (Variables|Default|GetDetectionDelay)))

(event Custom|DebugEvent
  (params (Debug :type Boolean))
  (if Debug
    (Development|SetHiddeninGame (Variables|Default|GetDetectionArea) false false)
    (Variables|Default|SetTraceDebug "ForOneFrame")
    (for (_array_element _array_index) (Variables|Default|GetWayPoints)
      (Rendering|Debug|DrawDebugSphere (Transformation|GetActorLocation _array_element) 3e+01 18 (Variables|Default|GetDebugColor) 99999999.0)
      (Rendering|Debug|DrawDebugLine (Transformation|GetActorLocation (Utilities|Array|Get(acopy) (Variables|Default|GetWayPoints) _array_index)) (Transformation|GetActorLocation (Utilities|Array|Get(acopy) (Variables|Default|GetWayPoints) (Math|Integer|%(Integer) (+ _array_index 1) (Utilities|Array|Length (Variables|Default|GetWayPoints))))) (Variables|Default|GetDebugColor) 99999999.0 5.0))
    (else
      (Development|SetHiddeninGame (Variables|Default|GetDetectionArea) true false)
      (Variables|Default|SetTraceDebug "None")
      (Class|KismetSystemLibrary|FlushDebugStrings)
      (Rendering|Debug|FlushPersistentDebugLines))))

(event EventBeginPlay
  (Utilities|FlowControl|Sequence
    (:then_0
      (bind _asfirst_person_game_mode (Utilities|Casting|CastToFirstPersonGameMode (Game|GetGameMode)))
      (Math|Integer|IncrementInt (Variables|/Game/Blueprints/FirstPersonGameMode.FirstPersonGameMode_C|GetEnemiesAlive _asfirst_person_game_mode)))
    (:then_1
      (bind _asfire_enemy_health (Utilities|Casting|CastToFireEnemyHealth (UserInterface|GetUserWidgetObject (Variables|Default|GetHealthBar))))
      (Variables|Default|SetHealthWidgetRef _asfire_enemy_health))
    (:then_2
      (Variables|Default|SetisLeft (Math|Random|RandomBool))
      (bind _outactors (Actor|GetAllActorsOfClass "/Script/Engine.TargetPoint"))
      (for _array_element _outactors
        (if (or (Utilities|String|Contains (Utilities|GetObjectName _array_element) "Left") (Utilities|String|Contains (Utilities|GetObjectName _array_element) "Right"))
          (if (or (and (Variables|Default|GetisLeft) (Utilities|String|Contains (Utilities|GetObjectName _array_element) "Left")) (and (Utilities|String|Contains (Utilities|GetObjectName _array_element) "Right") (not (Variables|Default|GetisLeft))))
            (Utilities|Array|Add (Variables|Default|GetWayPoints) _array_element :!label _label))
          (else
            (goto _label)))))))

(event Collision|EventActorBeginOverlap
  (params (OtherActor :type Actor%20Object%20Reference))
  ;[1 0.03917 0.07738] Detection Precess
  ;;[1 1 1] On Touch
  (Utilities|Casting|CastToFirstPersonCharacter OtherActor
    (:then
      (Variables|Default|SetIsInView true)
      (Variables|Default|SetDetectionDelayTemp (Variables|Default|GetDetectionDelay)))
    (:CastFailed
      (bind _asfirst_person_projectile (Utilities|Casting|CastToFirstPersonProjectile OtherActor))
      (if (not (Variables|/Game/Blueprints/FirstPersonProjectile.FirstPersonProjectile_C|GetisFire _asfirst_person_projectile))
        (Variables|Default|SetHealth (- (Variables|Default|GetHealth) (Variables|/Game/Blueprints/FirstPersonProjectile.FirstPersonProjectile_C|Getdamage _asfirst_person_projectile)))
        (Actor|DestroyActor _asfirst_person_projectile)))))

(event Collision|EventHit
  (params (MyComp :type Primitive%20Component%20Object%20Reference) (Other :type Actor%20Object%20Reference) (OtherComp :type Primitive%20Component%20Object%20Reference) (bSelfMoved :type Boolean) (HitLocation :type Vector :default "0, 0, 0") (HitNormal :type Vector :default "0, 0, 0") (NormalImpulse :type Vector :default "0, 0, 0") (Hit :type Hit%20Result%20Structure%20%28by%20ref%29))
  ;[1 0.03917 0.07738] Detection Precess
  ;;[1 1 1] On Touch
)

(event EventTick
  (params (DeltaSeconds :type Float%20%28single-precision%29))
  (bind _returnvalue (Game|Player|GetPlayerPawn 0))
  (bind _returnvalue_2 (Game|GetPlayerCharacter 0))
  (bind _health (Variables|Default|GetHealth))
  (bind _healthbar (Variables|Default|GetHealthBar))
  (bind _returnvalue_3 (Transformation|GetActorLocation _returnvalue_2))
  (bind _returnvalue_4 (Transformation|GetWorldLocation _healthbar))
  (bind _returnvalue_5 (Math|Rotator|FindLookatRotation _returnvalue_4 _returnvalue_3))
  ;[1 1 1] Tick
  (Utilities|FlowControl|Sequence
    (:then_0
      ;[1 0.03917 0.07738] Detection Precess
      (CallFunction|EyesTrace :!pinned true) ; Eyes Line Trace
    )
    (:then_1
      ;[1 0.6846 0.06277] Define AlertMode
      (Math|Float|CompareFloat (Variables|Default|GetDetectionDelayTemp) 0.0
        (:>
          (Variables|Default|SetDetectionDelayTemp (- (Variables|Default|GetDetectionDelayTemp) (Utilities|Time|GetWorldDeltaSeconds)))
          (bind _distance (CallFunction|GetDistancetoPlayer))
          (Math|Float|CompareFloat _distance (Variables|Default|GetAttackDistance)
            (:>
              (Variables|Default|SetAlertMode "NewEnumerator1"))
            (:==
              (Variables|Default|SetAlertMode "NewEnumerator0" :!label _label))
            (:<
              (goto _label))))
        (:==
          (if (Variables|Default|GetIsSupecious) :!label _label_2
            (Variables|Default|SetAlertMode "NewEnumerator2")
            (else
              (Variables|Default|SetAlertMode "NewEnumerator3"))))
        (:<
          (goto _label_2))))
    (:then_2
      ;[0.9166 1 0.0648] Switch On Alert Mode
      (switch Utilities|FlowControl|Switch|SwitchonEnum_AlertMode (Variables|Default|GetAlertMode)
        (:NewEnumerator0
          (CallFunction|ChangeSpeed (Variables|Default|GetAttackSpeed))
          (CallFunction|LookforSuspect)
          (Utilities|FlowControl|Sequence
            (:then_0
              (Utilities|FlowControl|Delay (Variables|Default|GetFireRate))
              (CallFunction|Attack))
            (:then_1
              (bind _distance_2 (CallFunction|GetDistancetoPlayer))
              (Math|Float|CompareFloat _distance_2 (Variables|Default|GetStopMovementDistance)
                (:>
                  (CallFunction|Chase))
                (:==
                  (Components|Movement|StopMovementImmediately :!label _label_3))
                (:<
                  (goto _label_3))))))
        (:NewEnumerator1
          (CallFunction|ChangeSpeed (Variables|Default|GetChaseSpeed))
          (CallFunction|LookforSuspect)
          (CallFunction|Chase))
        (:NewEnumerator2
          (CallFunction|ChangeSpeed (Variables|Default|GetSuspeciousSpeed))
          (CallFunction|LookforSuspect)
          (CallFunction|Patrol :!label _label_4))
        (:NewEnumerator3
          (CallFunction|ChangeSpeed (Variables|Default|GetPatrolSpeed))
          (CallFunction|ResetEyesRotation)
          (goto _label_4))))
    (:then_3
      ;[0 1 0.2061] Player Death
      (if (Utilities|IsValid _returnvalue)
        (bind _asfirst_person_character (Utilities|Casting|CastToFirstPersonCharacter _returnvalue))
        (if (Variables|/Game/Blueprints/FirstPersonCharacter.FirstPersonCharacter_C|GetisDead _asfirst_person_character)
          (Utilities|FlowControl|DoOnce false :!label _label_5
            (:Completed
              (Variables|Default|SetDetectionDelayTemp 0.1)))
          (else
            (goto _label_5 Reset)))))
    (:then_4
      ;[1 1 1] Enemy Death
      (Variables|/Game/Blueprints/FireEnemyHealth.FireEnemyHealth_C|SetNewVar_0 (Variables|Default|GetHealthWidgetRef) _health)
      (if (or (<= _health 0.0) (Math|Float|NearlyEqual(Float) _health 0.0 1e-06))
        ;;[1 0 0.07331] Update Wave
        (bind _asfirst_person_game_mode (Utilities|Casting|CastToFirstPersonGameMode (Game|GetGameMode))
          (:then
            (Math|Integer|DecrementInt (Variables|/Game/Blueprints/FirstPersonGameMode.FirstPersonGameMode_C|GetEnemiesAlive _asfirst_person_game_mode)
              (:%20%20
                (Default|CheckEnemiesLeft _asfirst_person_game_mode))))
          (:CastFailed
            (Development|PrintString "failed")))
        ;;[1 0 0.07331] Update Player Materials
        (bind _asfirst_person_character_2 (Utilities|Casting|CastToFirstPersonCharacter (Game|Player|GetPlayerPawn 0))
          (:then
            (Variables|/Game/Blueprints/FirstPersonCharacter.FirstPersonCharacter_C|SetMaterials _asfirst_person_character_2 (+ (Variables|/Game/Blueprints/FirstPersonCharacter.FirstPersonCharacter_C|GetMaterials _asfirst_person_character_2) 1)))
          (:CastFailed
            _))
        (Actor|DestroyActor)))
    (:then_5
      (Transformation|SetWorldRotation _healthbar (Math|Rotator|MakeRotator (.roll _returnvalue_5) (.pitch _returnvalue_5) (.yaw _returnvalue_5)) false false))))

(fn ConstructionScript
  (bind _detectionarea (Variables|Default|GetDetectionArea))
  (Transformation|SetRelativeLocation _detectionarea (Variables|Default|GetDetectionAreaRelativeLocation) false false)
  (Components|Box|SetBoxExtent _detectionarea (Variables|Default|GetDetectionAreaScale) true)
  (bind _returnvalue (Rendering|Material|CreateDynamicMaterialInstance (Variables|Character|GetMesh) 0 0 "None" :!class /Script/Engine.PrimitiveComponent))
  (Variables|Default|SetMaterialInstance _returnvalue))

(fn Patrol
  (if (and (<= (Transformation|GetHorizontalDistanceTo (Utilities|Array|Get(acopy) (Variables|Default|GetWayPoints) (Variables|Default|GetCurrentPoint))) 6e+01) (<= (Class|Actor|GetVerticalDistanceto (Utilities|Array|Get(acopy) (Variables|Default|GetWayPoints) (Variables|Default|GetCurrentPoint))) 1e+01))
    (if (>= (Variables|Default|GetCurrentPoint) (- (Utilities|Array|Length (Variables|Default|GetWayPoints)) 1))
      (bind _outactors (Actor|GetAllActorsOfClass "/Game/Blueprints/BP_Base.BP_Base_C"))
      (Variables|/Game/Blueprints/BP_Base.BP_Base_C|SetHealth (Utilities|Array|Get(acopy) _outactors) (- (Variables|/Game/Blueprints/BP_Base.BP_Base_C|GetHealth (Utilities|Array|Get(acopy) _outactors)) 0.2))
      (bind _asfirst_person_game_mode (Utilities|Casting|CastToFirstPersonGameMode (Game|GetGameMode))
        (:then
          (Math|Integer|DecrementInt (Variables|/Game/Blueprints/FirstPersonGameMode.FirstPersonGameMode_C|GetEnemiesAlive _asfirst_person_game_mode)
            (:%20%20
              (Default|CheckEnemiesLeft _asfirst_person_game_mode)
              (Actor|DestroyActor))))
        (:CastFailed
          (Development|PrintString "failed")))
      (else
        (Variables|Default|SetCurrentPoint (+ (Variables|Default|GetCurrentPoint) 1))))
    (else
      (AI|Navigation|SimpleMovetoActor (Pawn|GetController) (Utilities|Array|Get(acopy) (Variables|Default|GetWayPoints) (Variables|Default|GetCurrentPoint))))))

(fn Chase
  (AI|Navigation|SimpleMovetoActor (Pawn|GetController) (Game|Player|GetPlayerPawn 0)))

(fn Attack
  (bind _shooter (Variables|Default|GetShooter))
  (bind _returnvalue (Transformation|GetWorldLocation _shooter))
  (Game|SpawnActorfromClass "/Game/Blueprints/BP_ProjectileActor.BP_ProjectileActor_C" (Math|Transform|MakeTransform _returnvalue (Math|Rotator|FindLookatRotation _returnvalue (Transformation|GetActorLocation (Game|Player|GetPlayerPawn 0))) "0.300000,0.300000,0.300000") "AlwaysSpawn" 0 0))

(fn LookforSuspect
  (bind _eyes (Variables|Default|GetEyes))
  (Transformation|SetWorldRotation _eyes (Math|Rotator|FindLookatRotation (Transformation|GetWorldLocation _eyes) (Transformation|GetActorLocation (Game|Player|GetPlayerPawn 0))) true false))

(fn ResetEyesRotation
  (Transformation|SetRelativeRotation (Variables|Default|GetEyes) "0, 0, 0" true false))

(fn ChangeSpeed
  (params (NewSpeed :type Float%20%28single-precision%29))
  (Variables|/Script/Engine.CharacterMovementComponent|SetMaxWalkSpeed (Variables|Character|GetCharacterMovement) (Math|Float|Lerp NewSpeed (Variables|/Script/Engine.CharacterMovementComponent|GetMaxWalkSpeed (Variables|Character|GetCharacterMovement)) 0.85)))

(fn GetDistancetoPlayer
  (return (Transformation|GetDistanceTo (Game|Player|GetPlayerPawn 0))))

(fn EyesTrace
  (bind _eyes (Variables|Default|GetEyes))
  (bind _returnvalue (Transformation|GetWorldLocation _eyes))
  (bind _outhit (Collision|LineTraceByChannel _returnvalue (+ _returnvalue (* (Math|Vector|GetForwardVector _eyes) (Variables|Default|GetFieldOfView))) "TraceTypeQuery1" false 0 (Variables|Default|GetTraceDebug)))
  (bind _asfirst_person_character (Utilities|Casting|CastToFirstPersonCharacter (.HitActor (Collision|BreakHitResult _outhit)))
    (:then
      (if (Variables|/Game/Blueprints/FirstPersonCharacter.FirstPersonCharacter_C|GetisDead _asfirst_person_character)
        (Variables|Default|SetDetectionDelayTemp 0.0)
        (else
          (Variables|Default|SetIsInView true)
          (Variables|Default|SetDetectionDelayTemp (Variables|Default|GetDetectionDelay)))))
    (:CastFailed
      (Variables|Default|SetIsInView false))))