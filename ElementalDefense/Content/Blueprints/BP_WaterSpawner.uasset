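; BP_WaterSpawner is a wave spawner that creates BP_WaterDragon enemies around its location when the game mode starts a new wave.
; On BeginPlay it binds SpawnNextWave to the FirstPersonGameMode.
; A delayed loop spawns one dragon every half second at a random XY offset and fixed height.
; After each wave it raises EnemyIncrement and adds it to EnemiesSpawned, so waves grow progressively larger.
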(event Custom|SpawnNextWave
  (bind _returnvalue (Transformation|GetActorTransform))
  (bind _returnvalue_2 (Math|Random|RandomFloatinRange -2e+02 2e+02))
  (bind _variable (|TemporaryVariable))
  (|Assign _variable)
  (if (<= _variable (Variables|Default|GetEnemiesSpawned)) :!label _label
    (Utilities|FlowControl|Sequence
      (:then_0
        (Game|SpawnActorfromClass "/Game/Blueprints/BP_WaterDragon.BP_WaterDragon_C" (Math|Transform|MakeTransform (Math|Vector|MakeVector (+ _returnvalue_2 (.x (.location _returnvalue))) (+ _returnvalue_2 (.y (.location _returnvalue))) -3.9e+02) (.rotation _returnvalue) (.scale _returnvalue)) "AdjustIfPossibleButAlwaysSpawn" 0 0))
      (:then_1
        (Utilities|FlowControl|Delay 0.5)
        (|Assign _variable (+ _variable 1))
        (goto _label)))
    (else
      (bind _result (Math|Integer|IncrementInt (Variables|Default|GetEnemyIncrement))
        (:%20%20
          (Variables|Default|SetEnemiesSpawned (+ _result (Variables|Default|GetEnemiesSpawned))))))))

(event EventBeginPlay
  (bind _asfirst_person_game_mode (Utilities|Casting|CastToFirstPersonGameMode (Game|GetGameMode)))
  (EventDispatchers|BindEventtoSpawnNextWave _asfirst_person_game_mode (delegate Custom|SpawnNextWave)))

(fn ConstructionScript)