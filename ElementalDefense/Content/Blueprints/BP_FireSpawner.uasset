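; BP_FireSpawner is a wave spawner that creates fire or water dragons, picked at random, at its X/Y location and a fixed height.
; It binds to the FirstPersonGameMode next-wave event, waits an initial delay, then spawns enemies in a delayed loop.
; Each dragon receives the spawner's left-side and random-path flags before setting its waypoints.
; After each wave, the enemy count rises by an increment that itself grows, so waves escalate.
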(event Custom|SpawnNextWave
  (bind _returnvalue (Transformation|GetActorTransform))
  (bind _returnvalue_2 (Math|Random|RandomFloatinRange 0.0 0.0))
  (bind _variable (|TemporaryVariable))
  (bind _returnvalue_3 (+ _returnvalue_2 (.y (.location _returnvalue))))
  (bind _returnvalue_4 (+ _returnvalue_2 (.x (.location _returnvalue))))
  (Utilities|FlowControl|Delay (Variables|Default|GetInitialDelayPerWave))
  (|Assign _variable)
  (if (<= _variable (Variables|Default|GetEnemiesSpawned)) :!label _label
    (Utilities|FlowControl|Sequence
      (:then_0
        (if (Math|Random|RandomBool)
          (bind _returnvalue_5 (Game|SpawnActorfromClass "/Game/Blueprints/BP_FireDragon.BP_FireDragon_C" (Math|Transform|MakeTransform (Math|Vector|MakeVector _returnvalue_4 _returnvalue_3 -4e+02) (.rotation _returnvalue) "1,1,1") "AlwaysSpawn" 0 0))
          (Variables|/Game/Blueprints/BP_FireDragon.BP_FireDragon_C|SetisLeft _returnvalue_5 (Variables|Default|GetisLeftSpawner))
          (Variables|/Game/Blueprints/BP_FireDragon.BP_FireDragon_C|Setrandom _returnvalue_5 (Variables|Default|GetisRandomPath))
          (Default|SetWaypoints _returnvalue_5)
          (else
            (bind _returnvalue_6 (Game|SpawnActorfromClass "/Game/Blueprints/BP_WaterDragon.BP_WaterDragon_C" (Math|Transform|MakeTransform (Math|Vector|MakeVector _returnvalue_4 _returnvalue_3 -4e+02) "0, 0, 0" "1,1,1") "AlwaysSpawn" 0 0))
            (Variables|/Game/Blueprints/BP_WaterDragon.BP_WaterDragon_C|SetisLeft _returnvalue_6 (Variables|Default|GetisLeftSpawner))
            (Variables|/Game/Blueprints/BP_WaterDragon.BP_WaterDragon_C|Setrandom _returnvalue_6 (Variables|Default|GetisRandomPath))
            (Default|SetWaypoints _returnvalue_6))))
      (:then_1
        (Utilities|FlowControl|Delay (Variables|Default|GetDelayBetweenEnemies))
        (|Assign _variable (+ _variable 1))
        (goto _label)))
    (else
      (bind _result (Math|Integer|IncrementInt (Variables|Default|GetEnemyIncrement))
        (:%20%20
          (Variables|Default|SetEnemiesSpawned (+ _result (Variables|Default|GetEnemiesSpawned))))))))

(event EventBeginPlay
  (bind _asfirst_person_game_mode (Utilities|Casting|CastToFirstPersonGameMode (Game|GetGameMode)))
  (EventDispatchers|BindEventtoSpawnNextWave _asfirst_person_game_mode (delegate Custom|SpawnNextWave)))

(fn ConstructionScript)