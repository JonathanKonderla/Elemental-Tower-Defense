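; Enemy spawner actor that creates escalating waves of water dragons.
; On BeginPlay it binds to the SpawnNextWave event dispatcher on FirstPersonGameMode.
; Each wave spawns the current count of BP_WaterDragon at the spawner's transform, with height fixed at a negative Z.
; It then raises the increment and adds it to the count, so wave sizes grow faster than linearly.
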(event Custom|SpawnNextWave
  (bind _returnvalue (Transformation|GetActorTransform))
  (for _index (range 1 (Variables|Default|GetEnemiesSpawned))
    (Game|SpawnActorfromClass "/Game/Blueprints/BP_WaterDragon.BP_WaterDragon_C" (Math|Transform|MakeTransform (Math|Vector|MakeVector (.x (.location _returnvalue)) (.y (.location _returnvalue)) -4e+02) (.rotation _returnvalue) (.scale _returnvalue)) "Undefined" 0 0))
  (bind _result (Math|Integer|IncrementInt (Variables|Default|GetEnemyIncrement))
    (:%20%20
      (Variables|Default|SetEnemiesSpawned (+ _result (Variables|Default|GetEnemiesSpawned))))))

(event EventBeginPlay
  (bind _asfirst_person_game_mode (Utilities|Casting|CastToFirstPersonGameMode (Game|GetGameMode)))
  (EventDispatchers|BindEventtoSpawnNextWave _asfirst_person_game_mode (delegate Custom|SpawnNextWave)))

(fn ConstructionScript)