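; Character Blueprint that tracks the player character's health and handles its death and respawn.
; Any damage reduces health, and at zero the character is flagged dead, with gravity and collision disabled and the mesh hidden rather than the actor being destroyed.
; A Respawn event reverses those changes and restores full health on the same actor, without moving it.
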(event Custom|Respawn
  (Collision|SetActorEnableCollision true)
  (Rendering|SetVisibility (Variables|Character|GetMesh) true true)
  (Variables|/Script/Engine.CharacterMovementComponent|SetGravityScale (Variables|Character|GetCharacterMovement) 1.0)
  (Variables|Default|SetHealth 1e+02)
  (Variables|Default|SetIsDead false))

(event Game|Damage|EventAnyDamage
  (params (Damage :type Float%20%28single-precision%29) (DamageType :type Damage%20Type%20Object%20Reference) (InstigatedBy :type Controller%20Object%20Reference) (DamageCauser :type Actor%20Object%20Reference))
  ;[1 1 1] Damage / Death
  (Variables|Default|SetHealth (- (Variables|Default|GetHealth) Damage))
  (if (<= (Variables|Default|GetHealth) 0.0)
    (Variables|Default|SetHealth 0.0)
    (Variables|Default|SetIsDead true)
    (Variables|/Script/Engine.CharacterMovementComponent|SetGravityScale (Variables|Character|GetCharacterMovement) 0.0)
    (Collision|SetActorEnableCollision false)
    (Rendering|SetVisibility (Variables|Character|GetMesh) false false)))

(event EventBeginPlay
  ;[1 1 1] Begin Play
  (Variables|Default|SetHealth 1e+02)
  (Variables|Default|SetIsDead false))

(fn ConstructionScript)